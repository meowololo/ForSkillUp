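; BP_Bonus1 is a falling Arkanoid bonus pickup that widens the player's platform when caught.
; BeginPlay sizes and rotates the pickup, then Tick sweeps the Ere2 component downward by a fixed per-frame offset, independent of delta time.
; On overlap with the platform pawn it increases that pawn's Y scale.
; Either that overlap or hitting a KillZVolume destroys Ere2 and sets IsDead, halting movement while the actor itself remains.
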(event `self.ReceiveBeginPlay`
  (`SceneComponent.K2_SetWorldRotation` (`self.ere2`) (struct :`Pitch` 90.0 :`Yaw` 90.0) false false)
  (`self.SetActorScale3D` (0.625 1.5 0.125)))

(event `self.ReceiveTick`
  (params (DeltaSeconds :type "Float (single-precision)"))
  (if (not (`self.isDead?`))
    (`SceneComponent.K2_AddWorldOffset` (`self.ere2`) (* (* (0.0 0.0 -90.0) 3.0) 0.015) true false)))

(event `self.ReceiveActorBeginOverlap`
  (params (OtherActor :type "Actor Object Reference"))
  (bind _aspawn_arkanoid_platform (cast `/Game/Skill/Pawn_ArkanoidPlatform` OtherActor)
    (:`then`
      (bind (_returnvalue_x _returnvalue_y _returnvalue_z) (`KismetMathLibrary.BreakVector` (`self.GetActorScale3D` _aspawn_arkanoid_platform)))
      (`self.SetActorScale3D` _aspawn_arkanoid_platform (`KismetMathLibrary.MakeVector` _returnvalue_x (+ _returnvalue_y 1.0) _returnvalue_z))
      (`ActorComponent.K2_DestroyComponent` (`self.ere2`)))
    (:`CastFailed`
      (cast `KillZVolume` OtherActor)
      (`ActorComponent.K2_DestroyComponent` (`self.ere2`))))
  (set `self.isDead?` true))

(fn `UserConstructionScript`)