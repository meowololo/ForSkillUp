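; Breakable block for an Arkanoid-style game that takes two hits from an ArcanoidBall and can drop a bonus.
; The first hit sets a flag and swaps the hit component's material, and the next hit destroys the block.
; A random MultiGate serves as a weighted drop roll: most outputs only destroy the block, while three first spawn one of three bonus actors at the cube's location.
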(event `self.ReceiveHit`
  (params (MyComp :type "PrimitiveComponent Object Reference") (Other :type "Actor Object Reference") (OtherComp :type "PrimitiveComponent Object Reference") (bSelfMoved :type Boolean) (HitLocation :type "Vector Structure") (HitNormal :type "Vector Structure") (NormalImpulse :type "Vector Structure") (Hit :type "HitResult Structure (by ref)"))
  (cast `/Game/Skill/ArcanoidBall` Other)
  (if (`self.wasHit`)
    (`|MultiGate` true true
      (:`Out 0`
        (`self.K2_DestroyActor` :!label _label))
      (:`Out 1`
        (goto _label))
      (:`Out 2`
        (goto _label))
      (:`Out 3`
        (goto _label))
      (:`Out 4`
        (goto _label))
      (:`Out 5`
        (goto _label))
      (:`Out 6`
        (goto _label))
      (:`Out 7`
        (goto _label))
      (:`Out 8`
        (goto _label))
      (:`Out 9`
        (goto _label))
      (:`Out 10`
        (goto _label))
      (:`Out 11`
        (goto _label))
      (:`Out 12`
        (goto _label))
      (:`Out 13`
        (`|SpawnActorFromClass` "/Game/Skill/BP_Bonus1.BP_Bonus1_C" (`KismetMathLibrary.Conv_VectorToTransform` (`SceneComponent.K2_GetComponentLocation` (`self.Cube`))) "AlwaysSpawn" "OverrideRootScale" null null)
        (`self.K2_DestroyActor`))
      (:`Out 14`
        (`|SpawnActorFromClass` "/Game/Skill/BP_Bonus2.BP_Bonus2_C" (`KismetMathLibrary.Conv_VectorToTransform` (`SceneComponent.K2_GetComponentLocation` (`self.Cube`))) "AlwaysSpawn" "OverrideRootScale" null null)
        (`self.K2_DestroyActor`))
      (:`Out 15`
        (`|SpawnActorFromClass` "/Game/Skill/BP_Bonus3.BP_Bonus3_C" (`KismetMathLibrary.Conv_VectorToTransform` (`SceneComponent.K2_GetComponentLocation` (`self.Cube`))) "Undefined" "OverrideRootScale" null null)
        (`self.K2_DestroyActor`)))
    (else
      (`PrimitiveComponent.SetMaterial` MyComp 0 "/Game/Colors/LightColorBasic.LightColorBasic")
      (set `self.wasHit` true))))

(fn `UserConstructionScript`)